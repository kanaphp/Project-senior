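; Trigger actor in the Singburi province area that shows the Shop C info actor while it is overlapped.
; Actor overlap passes through a DoOnce and spawns BP_InfoShopC at a fixed world-space offset from the Box, matching its rotation.
; Ending overlap on the Box destroys that actor and resets the DoOnce for the next entry.
; Neither event filters which actor overlaps.
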(event `self.ReceiveActorBeginOverlap`
  (params (OtherActor :type "Actor Object Reference"))
  (bind _box (`self.Box`))
  (`/Engine/EditorBlueprintResources/StandardMacros.DoOnce` false :!label _label
    (:`Completed`
      (bind _returnvalue (`|SpawnActorFromClass` "/Game/MyGame/Province/Singburi/Blueprints/BP_InfoShopC.BP_InfoShopC_C" (`KismetMathLibrary.MakeTransform` (+ (`SceneComponent.K2_GetComponentLocation` _box) (-60.0 60.0 150.0)) (`SceneComponent.K2_GetComponentRotation` _box)) "Undefined" "MultiplyWithRoot" null null))
      (set `self.WgShop` _returnvalue))))

(event `self.Box.OnComponentEndOverlap`
  (params (OverlappedComponent :type "PrimitiveComponent Object Reference") (OtherActor :type "Actor Object Reference") (OtherComp :type "PrimitiveComponent Object Reference") (OtherBodyIndex :type Integer))
  (`self.K2_DestroyActor` (`self.WgShop`))
  (goto _label :!via `Reset`))

(fn `UserConstructionScript`)