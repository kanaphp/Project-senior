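; Manager for the Singburi province minigame, running the time-limited target spawning and the end screen actor.
; While running, StartMinigame re-arms itself on a one-second timer, counts down RemainTime and triggers SpawnTarget through a delay.
; SpawnTarget places random target classes at randomly picked, non-repeating BP_SpawnPoint actors.
; At zero it spawns BP_MinigameSingburiEnd, which Tick destroys once flagged closed; the widget and win-flag logic is disconnected.
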(event `self.ReceiveBeginPlay`)

(event `StartMinigame`
  ; Counntdown timelimit minigame
  (if (`self.isRunning`)
    (`KismetSystemLibrary.K2_SetTimerDelegate` (delegate `StartMinigame`) 1.0)
    (if (== (`self.RemainTime`) 0)
      ; Stop spawn and show end widget
      (set `self.isRunning` false)
      (`|SpawnActorFromClass` "/Game/MyGame/Province/Singburi/Blueprints/BP_MinigameSingburiEnd.BP_MinigameSingburiEnd_C" (`KismetMathLibrary.MakeTransform` (+ (1600.0 -900.0 65.0) (100.0 -100.0 100.0)) (`self.K2_GetActorRotation`) (0.6 0.6 0.6)) "Undefined" "MultiplyWithRoot" null null)
      (else
        ; Spawn target
        (set `self.RemainTime` (- (`self.RemainTime`) 1))
        (`KismetSystemLibrary.Delay` 5.0)
        (`self.SpawnTarget`)))))

(event `self.ReceiveTick`
  (params (DeltaSeconds :type "Float (single-precision)"))
  (bind _returnvalue (`GameplayStatics.GetActorOfClass` "/Game/MyGame/Province/Singburi/Blueprints/BP_MinigameSingburiEnd.BP_MinigameSingburiEnd_C"))
  (set `self.endMinigame` _returnvalue)
  (`/Engine/EditorBlueprintResources/StandardMacros.IsValid` _returnvalue
    (:`Is Valid`
      (if (`/Game/MyGame/Province/Singburi/Blueprints/BP_MinigameSingburiEnd.isClose` _returnvalue)
        (`/Engine/EditorBlueprintResources/StandardMacros.DoOnce` false
          (:`Completed`
            (`self.K2_DestroyActor` (`self.endMinigame`))))))))

(fn `SpawnTarget`
  (locals (LocalSpawnReferences :type "Array of /Game/MyGame/Province/Singburi/Blueprints/BP_SpawnPoint Object Reference") (LocalItem :type "/Game/MyGame/Province/Singburi/Blueprints/BP_SpawnPoint Object Reference"))
  (`KismetSystemLibrary.PrintString` "Hello spawntarget activate")
  (bind _outactors (`GameplayStatics.GetAllActorsOfClass` "/Game/MyGame/Province/Singburi/Blueprints/BP_SpawnPoint.BP_SpawnPoint_C"))
  (set `local.LocalSpawnReferences` _outactors)
  (for _ (range (`self.MaxSpawn`))
    (set `local.LocalItem` (`KismetArrayLibrary.Array_Random` (`local.LocalSpawnReferences`)))
    (`|SpawnActorFromClass` (`KismetArrayLibrary.Array_Random` (`self.AllTarget`)) (`KismetMathLibrary.MakeTransform` (`self.K2_GetActorLocation` (`local.LocalItem`)) (struct :`Yaw` 55.0)) "Undefined" "MultiplyWithRoot" null null)
    (`KismetSystemLibrary.PrintString` "spawn!!")
    (`KismetArrayLibrary.Array_RemoveItem` (`local.LocalSpawnReferences`) (`local.LocalItem`))))

(fn `UserConstructionScript`)