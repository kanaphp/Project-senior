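; BP_TriggerMinigame is a trigger actor that shows the Singburi minigame actor while something overlaps it.
; Actor begin overlap passes a DoOnce and spawns BP_MinigameSingburi at reduced scale, offset from the Box, storing it in WgMinigame.
; Box end overlap destroys that actor and resets the DoOnce, with no check on which actor overlaps.
; Unconnected leftover nodes would instead toggle an MG_MinigameSingburi viewport widget, mouse cursor and input mode.
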(event `self.ReceiveActorBeginOverlap`
  (params (OtherActor :type "Actor Object Reference"))
  (`/Engine/EditorBlueprintResources/StandardMacros.DoOnce` false :!label _label
    (:`Completed`
      (bind _returnvalue (`|SpawnActorFromClass` "/Game/MyGame/Province/Singburi/Blueprints/BP_MinigameSingburi.BP_MinigameSingburi_C" (`KismetMathLibrary.MakeTransform` (+ (`SceneComponent.K2_GetComponentLocation` (`self.Box`)) (100.0 -100.0 100.0)) (`self.K2_GetActorRotation`) (0.6 0.6 0.6)) "Undefined" "MultiplyWithRoot" null null))
      (set `self.wgMinigame` _returnvalue))))

(event `self.Box.OnComponentEndOverlap`
  (params (OverlappedComponent :type "PrimitiveComponent Object Reference") (OtherActor :type "Actor Object Reference") (OtherComp :type "PrimitiveComponent Object Reference") (OtherBodyIndex :type Integer))
  (`self.K2_DestroyActor` (`self.wgMinigame`))
  (goto _label :!via `Reset`))

(fn `UserConstructionScript`)