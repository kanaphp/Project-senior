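; BP_TriggerWatpho is a trigger actor that shows a BP_InfoWatpho information actor when something overlaps it.
; On first overlap, a DoOnce spawns the info actor at a fixed offset from the Box, rotated to the player character's facing, and stores it.
; When the Box overlap ends, it destroys that actor and resets the DoOnce so the info can appear again.
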(event `self.ReceiveActorBeginOverlap`
  (params (OtherActor :type "Actor Object Reference"))
  (`/Engine/EditorBlueprintResources/StandardMacros.DoOnce` false :!label _label
    (:`Completed`
      (bind _returnvalue (`|SpawnActorFromClass` "/Game/MyGame/Province/Singburi/Blueprints/BP_InfoWatpho.BP_InfoWatpho_C" (`KismetMathLibrary.MakeTransform` (+ (`SceneComponent.K2_GetComponentLocation` (`self.Box`)) (50.0 -50.0 150.0)) (`self.K2_GetActorRotation` (`GameplayStatics.GetPlayerCharacter` 0))) "Undefined" "MultiplyWithRoot" null null))
      (set `self.wg_watpho` _returnvalue))))

(event `self.Box.OnComponentEndOverlap`
  (params (OverlappedComponent :type "PrimitiveComponent Object Reference") (OtherActor :type "Actor Object Reference") (OtherComp :type "PrimitiveComponent Object Reference") (OtherBodyIndex :type Integer))
  (`self.K2_DestroyActor` (`self.wg_watpho`))
  (goto _label :!via `Reset`))

(fn `UserConstructionScript`)