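; BP_InfoFish is an actor in the Singburi province content that routes VR menu input to the player's widget pointers.
; On BeginPlay it caches the VRPawn, enables its tick, enables input on itself and adds IMC_Default to the local player.
; Left and right menu-interact actions press LeftMouseButton on the matching WidgetInteraction component when triggered and release it when completed or canceled.
; It contains no fish-specific logic in its graphs.
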(event `self.ReceiveBeginPlay`
  (bind _returnvalue (`GameplayStatics.GetPlayerController` 0))
  (bind _asvrpawn (cast `/Game/VRTemplate/Blueprints/VRPawn` (`GameplayStatics.GetPlayerPawn` 0)))
  (bind _output_get (set `self.VRPawn` _asvrpawn))
  (`self.SetActorTickEnabled` _output_get true)
  (`self.EnableInput` _returnvalue)
  (`EnhancedInputSubsystemInterface.AddMappingContext` (pcsubsystem `EnhancedInputLocalPlayerSubsystem` _returnvalue) "/Game/VRTemplate/Input/IMC_Default.IMC_Default" 1 (struct)))

(event `EnhancedInput|/Game/VRTemplate/Input/Actions/IA_Menu_Interact_Left_Pressed`
  (params (ActionValue :type Boolean) (ElapsedSeconds :type "Float (double-precision)") (TriggeredSeconds :type "Float (double-precision)") (InputAction :type "InputAction Object Reference" :default "/Game/VRTemplate/Input/Actions/IA_Menu_Interact_Left_Pressed.IA_Menu_Interact_Left_Pressed"))
  (bind _widgetinteractionleft (`/Game/VRTemplate/Blueprints/VRPawn.WidgetInteractionLeft` (`self.VRPawn`)))
  (:`Triggered`
    (`WidgetInteractionComponent.PressPointerKey` _widgetinteractionleft "LeftMouseButton"))
  (:`Canceled`
    (`WidgetInteractionComponent.ReleasePointerKey` _widgetinteractionleft "LeftMouseButton" :!label _label))
  (:`Completed`
    (goto _label)))

(event `EnhancedInput|/Game/VRTemplate/Input/Actions/IA_Menu_Interact_Right_Pressed`
  (params (ActionValue :type Boolean) (ElapsedSeconds :type "Float (double-precision)") (TriggeredSeconds :type "Float (double-precision)") (InputAction :type "InputAction Object Reference" :default "/Game/VRTemplate/Input/Actions/IA_Menu_Interact_Right_Pressed.IA_Menu_Interact_Right_Pressed"))
  (bind _widgetinteractionright (`/Game/VRTemplate/Blueprints/VRPawn.WidgetInteractionRight` (`self.VRPawn`)))
  (:`Triggered`
    (`WidgetInteractionComponent.PressPointerKey` _widgetinteractionright "LeftMouseButton"))
  (:`Canceled`
    (`WidgetInteractionComponent.ReleasePointerKey` _widgetinteractionright "LeftMouseButton" :!label _label_2))
  (:`Completed`
    (goto _label_2)))

(fn `UserConstructionScript`)