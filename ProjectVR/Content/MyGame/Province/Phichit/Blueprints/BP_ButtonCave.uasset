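; BP_ButtonCave is a pressure button that signals a secret door to open when the first-person character steps into its box trigger.
; On overlap it plays a press sound through a DoOnce, lowers the button slightly and calls OpenSecretDoor.
; Ending the overlap moves the button back to the position stored at BeginPlay and resets the sound gate, with no signal to close the door.
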(event `self.ReceiveBeginPlay`
  (set `self.ButtonStart` (`SceneComponent.RelativeLocation` (`self.Button`))))

(event `self.Box.OnComponentBeginOverlap`
  (params (OverlappedComponent :type "PrimitiveComponent Object Reference") (OtherActor :type "Actor Object Reference") (OtherComp :type "PrimitiveComponent Object Reference") (OtherBodyIndex :type Integer) (bFromSweep :type Boolean) (SweepResult :type "HitResult Structure (by ref)"))
  (cast `/Game/FirstPerson/Blueprints/BP_FirstPersonCharacter` OtherActor)
  (`|ExecutionSequence`
    (:`then_0`
      (`/Engine/EditorBlueprintResources/StandardMacros.DoOnce` false :!label _label
        (:`Completed`
          (`GameplayStatics.PlaySound2D` "/Game/MyGame/Sound/PressButton.PressButton" 1.0 1.0 0.0 null null))))
    (:`then_1`
      (`KismetSystemLibrary.MoveComponentTo` (`self.Button`) (- (`self.ButtonStart`) (0.0 0.0 5.0)))
      (`KismetSystemLibrary.PrintString` "OpenSecretDoor")
      (`self.OpenSecretDoor`))))

(event `self.Box.OnComponentEndOverlap`
  (params (OverlappedComponent :type "PrimitiveComponent Object Reference") (OtherActor :type "Actor Object Reference") (OtherComp :type "PrimitiveComponent Object Reference") (OtherBodyIndex :type Integer))
  (cast `/Game/FirstPerson/Blueprints/BP_FirstPersonCharacter` OtherActor)
  (`KismetSystemLibrary.MoveComponentTo` (`self.Button`) (`self.ButtonStart`))
  (goto _label :!via `Reset`))

(fn `UserConstructionScript`)