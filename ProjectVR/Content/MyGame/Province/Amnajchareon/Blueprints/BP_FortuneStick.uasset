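; Fortune stick shaker that, when shaken long enough, ejects a stick and shows one of six random fortunes.
; Tick uses a one-second Delay to poll the object's physics velocity; movement jiggles five stick components, plays a shake sound and increments a counter, while stillness resets it.
; At the threshold, it spawns a short-lived physics stick and a fortune info actor oriented to the player's rotation, and adds an audio component.
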(event `Shake`
  (bind _stick (`self.Stick`))
  (bind _stick1 (`self.Stick1`))
  (bind _stick2 (`self.Stick2`))
  (bind _stick3 (`self.Stick3`))
  (bind _stick4 (`self.Stick4`))
  (`|ExecutionSequence`
    (:`then_0`
      (`KismetSystemLibrary.MoveComponentTo` _stick (-40.0 0.0 0.0) (struct :`Roll` -10.0))
      (`KismetSystemLibrary.MoveComponentTo` _stick (-40.0 0.0 0.0)))
    (:`then_1`
      (`KismetSystemLibrary.MoveComponentTo` _stick1 (0.0 -20.0 0.0) (struct :`Roll` -15.0))
      (`KismetSystemLibrary.MoveComponentTo` _stick1 (0.0 -20.0 0.0)))
    (:`then_2`
      (`KismetSystemLibrary.MoveComponentTo` _stick2 (40.0 -40.0 0.0) (struct :`Roll` -10.0))
      (`KismetSystemLibrary.MoveComponentTo` _stick2 (40.0 -40.0 0.0)))
    (:`then_3`
      (`KismetSystemLibrary.MoveComponentTo` _stick3 (-20.0 40.0 0.0) (struct :`Roll` -10.0))
      (`KismetSystemLibrary.MoveComponentTo` _stick3 (-20.0 40.0 0.0)))
    (:`then_4`
      (`KismetSystemLibrary.MoveComponentTo` _stick4 (40.0 20.0 0.0) (struct :`Roll` -10.0))
      (`KismetSystemLibrary.MoveComponentTo` _stick4 (40.0 20.0 0.0)))))

(event `self.ReceiveBeginPlay`)

(event `self.ReceiveTick`
  (params (DeltaSeconds :type "Float (single-precision)"))
  (`KismetSystemLibrary.Delay` 1.0)
  (bind _returnvalue (`PrimitiveComponent.GetPhysicsLinearVelocity` (`self.Object`) "None"))
  (if (!= _returnvalue (0.0 0.0 0.0))
    (`self.Shake`)
    (set `self.TimeShake` (+ (`self.TimeShake`) 1))
    (`GameplayStatics.SpawnSoundAttached` "/Game/MyGame/Province/Amnajchareon/Sound/SFX_Shake.SFX_Shake" (`self.Object`) "None" (0.0 0.0 0.0) (struct) "KeepRelativeOffset" false 1.0 1.0 0.0 null null)
    (if (>= (`self.TimeShake`) (`self.TimeShakeCheck`))
      (`self.PopoutFortune`)
      (bind _returnvalue_2 (`|SpawnActorFromClass` "/Game/MyGame/Province/Amnajchareon/Blueprints/BP_FortuneStickPop.BP_FortuneStickPop_C" (`KismetMathLibrary.Conv_VectorToTransform` (`SceneComponent.K2_GetComponentLocation` (`self.Object`))) "Undefined" "MultiplyWithRoot" null null))
      (bind _output_get (set `self.PopoutStick` _returnvalue_2))
      (`PrimitiveComponent.SetSimulatePhysics` (`/Game/MyGame/Province/Amnajchareon/Blueprints/BP_FortuneStickPop.PopStick` _output_get) true)
      (`self.SetLifeSpan` _output_get 5.0))
    (else
      (set `self.TimeShake` 0))))

(event `PopoutFortune`
  (set `self.FortuneNumber` (`KismetMathLibrary.RandomIntegerInRange` 0 5))
  (set `self.TimeShake` 0)
  (switch `int` (`self.FortuneNumber`)
    (:`0`
      (`self.SpawnFortune0`))
    (:`1`
      (`self.SpawnFortune1`))
    (:`2`
      (`self.SpawnFortune2`))
    (:`3`
      (`self.SpawnFortune3`))
    (:`4`
      (`self.SpawnFortune4`))
    (:`5`
      (`self.SpawnFortune5`)))
  (`AddComponent|NODE_AddAudioComponent-6`))

(event `SpawnFortune1`
  (bind _returnvalue (`|SpawnActorFromClass` "/Game/MyGame/Province/Amnajchareon/Blueprints/BP_InfoFortune1.BP_InfoFortune1_C" (`KismetMathLibrary.MakeTransform` (+ (+ (`SceneComponent.K2_GetComponentLocation` (`self.Object`)) (* (`self.GetActorForwardVector`) (`self.Distance`))) (-250.0 25.0 60.0)) (`self.K2_GetActorRotation` (`GameplayStatics.GetPlayerCharacter` 0))) "Undefined" "MultiplyWithRoot" null null))
  (`self.SetLifeSpan` _returnvalue 3.0))

(event `SpawnFortune4`
  (bind _returnvalue (`|SpawnActorFromClass` "/Game/MyGame/Province/Amnajchareon/Blueprints/BP_InfoFortune4.BP_InfoFortune4_C" (`KismetMathLibrary.MakeTransform` (+ (+ (`SceneComponent.K2_GetComponentLocation` (`self.Object`)) (* (`self.GetActorForwardVector`) (`self.Distance`))) (-250.0 25.0 60.0)) (`self.K2_GetActorRotation` (`GameplayStatics.GetPlayerCharacter` 0))) "Undefined" "MultiplyWithRoot" null null))
  (`self.SetLifeSpan` _returnvalue 3.0))

(event `SpawnFortune2`
  (bind _returnvalue (`|SpawnActorFromClass` "/Game/MyGame/Province/Amnajchareon/Blueprints/BP_InfoFortune2.BP_InfoFortune2_C" (`KismetMathLibrary.MakeTransform` (+ (+ (`SceneComponent.K2_GetComponentLocation` (`self.Object`)) (* (`self.GetActorForwardVector`) (`self.Distance`))) (-250.0 25.0 60.0)) (`self.K2_GetActorRotation` (`GameplayStatics.GetPlayerCharacter` 0))) "Undefined" "MultiplyWithRoot" null null))
  (`self.SetLifeSpan` _returnvalue 3.0))

(event `SpawnFortune5`
  (bind _returnvalue (`|SpawnActorFromClass` "/Game/MyGame/Province/Amnajchareon/Blueprints/BP_InfoFortune5.BP_InfoFortune5_C" (`KismetMathLibrary.MakeTransform` (+ (+ (`SceneComponent.K2_GetComponentLocation` (`self.Object`)) (* (`self.GetActorForwardVector`) (`self.Distance`))) (-250.0 25.0 60.0)) (`self.K2_GetActorRotation` (`GameplayStatics.GetPlayerCharacter` 0))) "Undefined" "MultiplyWithRoot" null null))
  (`self.SetLifeSpan` _returnvalue 3.0))

(event `SpawnFortune3`
  (bind _returnvalue (`|SpawnActorFromClass` "/Game/MyGame/Province/Amnajchareon/Blueprints/BP_InfoFortune3.BP_InfoFortune3_C" (`KismetMathLibrary.MakeTransform` (+ (+ (`SceneComponent.K2_GetComponentLocation` (`self.Object`)) (* (`self.GetActorForwardVector`) (`self.Distance`))) (-250.0 25.0 60.0)) (`self.K2_GetActorRotation` (`GameplayStatics.GetPlayerCharacter` 0))) "Undefined" "MultiplyWithRoot" null null))
  (`self.SetLifeSpan` _returnvalue 3.0))

(event `SpawnFortune0`
  (bind _returnvalue (`|SpawnActorFromClass` "/Game/MyGame/Province/Amnajchareon/Blueprints/BP_InfoFortune0.BP_InfoFortune0_C" (`KismetMathLibrary.MakeTransform` (+ (+ (`SceneComponent.K2_GetComponentLocation` (`self.Object`)) (* (`self.GetActorForwardVector`) (`self.Distance`))) (-250.0 25.0 60.0)) (`self.K2_GetActorRotation` (`GameplayStatics.GetPlayerCharacter` 0))) "Undefined" "MultiplyWithRoot" null null))
  (`self.SetLifeSpan` _returnvalue 3.0))

(fn `UserConstructionScript`)