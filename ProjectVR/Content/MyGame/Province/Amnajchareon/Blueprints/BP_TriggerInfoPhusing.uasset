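; Trigger actor in the Amnajchareon province content that shows the Phusing info actor with its 2D audio while overlapped.
; Actor overlap spawns BP_InfoPhusing once, offset along the trigger's forward vector by Distance, raised, and rotated to match the player character.
; Leaving the Box destroys that actor, stops the sound and resets the DoOnce for re-entry.
; Neither overlap event filters the overlapping actor.
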(event `self.ReceiveActorBeginOverlap`
  (params (OtherActor :type "Actor Object Reference"))
  ; Make Widget spawn distance to player
  (`/Engine/EditorBlueprintResources/StandardMacros.DoOnce` false :!label _label
    (:`Completed`
      (bind _returnvalue (`|SpawnActorFromClass` "/Game/MyGame/Province/Amnajchareon/Blueprints/BP_InfoPhusing.BP_InfoPhusing_C" (`KismetMathLibrary.MakeTransform` (+ (+ (`self.K2_GetActorLocation`) (* (`self.GetActorForwardVector`) (`self.Distance`))) (0.0 0.0 160.0)) (`self.K2_GetActorRotation` (`GameplayStatics.GetPlayerCharacter` 0))) "Undefined" "MultiplyWithRoot" null null))
      (set `self.WG_Info` _returnvalue)
      (bind _returnvalue_2 (`GameplayStatics.SpawnSound2D` "/Game/MyGame/Province/Amnajchareon/Sound/InfoPhusing.InfoPhusing" 1.0 1.0 0.0 null))
      (set `self.SoundInfo` _returnvalue_2))))

(event `self.Box.OnComponentEndOverlap`
  (params (OverlappedComponent :type "PrimitiveComponent Object Reference") (OtherActor :type "Actor Object Reference") (OtherComp :type "PrimitiveComponent Object Reference") (OtherBodyIndex :type Integer))
  ; Make Widget spawn distance to player
  (`self.K2_DestroyActor` (`self.WG_Info`))
  (`AudioComponent.Stop` (`self.SoundInfo`))
  (goto _label :!via `Reset`))

(fn `UserConstructionScript`)