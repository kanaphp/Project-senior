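; BP_Incense is an incense actor whose smoke stays hidden until it is lit.
; On BeginPlay it hides the smoke and binds its Light event to the LightUp dispatcher of the BP_LightTrigger found in the level.
; Light reveals the smoke and swaps the Burnn mesh to a black material to show burning.
; A separate CancelPhysic event turns off physics simulation on the Object component.
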(event `CancelPhysic`
  (`PrimitiveComponent.SetSimulatePhysics` (`self.Object`) false))

(event `self.ReceiveBeginPlay`
  (`SceneComponent.SetVisibility` (`self.Smoke`) false false)
  (bind _returnvalue (`GameplayStatics.GetActorOfClass` "/Game/MyGame/Province/Amnajchareon/Blueprints/BP_LightTrigger.BP_LightTrigger_C"))
  (add `/Game/MyGame/Province/Amnajchareon/Blueprints/BP_LightTrigger.LightUp` _returnvalue (delegate `Light`)))

(event `Light`
  (`SceneComponent.SetVisibility` (`self.Smoke`) true false)
  (`PrimitiveComponent.SetMaterial` (`self.Burnn`) 0 "/Game/MyGame/Province/Amnajchareon/Assets/Pramongkol/Materials/Black.Black"))

(fn `UserConstructionScript`)