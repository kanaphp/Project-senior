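; BP_CorrectTarget is a shootable target in the Singburi game that awards points when hit and removes itself after a short lifespan.
; The first hit on its Box adds a fixed score to ScoreSingburi in GI_MyGame, prints the total and plays the TargetSlowFall timeline.
; The timeline sets Pivot to zero rotation, leaving its Slowdown track unconnected, and destroys the actor after a brief delay.
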(event `self.ReceiveBeginPlay`
  (`self.SetLifeSpan` 4.5))

(event `self.Box.OnComponentHit`
  (params (HitComponent :type "PrimitiveComponent Object Reference") (OtherActor :type "Actor Object Reference") (OtherComp :type "PrimitiveComponent Object Reference") (NormalImpulse :type "Vector Structure") (Hit :type "HitResult Structure (by ref)"))
  ; Target slow fall when get shot and destroy and get score
  (bind _asgi_my_game (cast `/Game/MyGame/GI_MyGame` (`GameplayStatics.GetGameInstance`)))
  (`/Engine/EditorBlueprintResources/StandardMacros.DoOnce` false
    (:`Completed`
      (bind _output_get (set `/Game/MyGame/GI_MyGame.ScoreSingburi` (+ (`/Game/MyGame/GI_MyGame.ScoreSingburi` _asgi_my_game) 20) _asgi_my_game))
      (`KismetSystemLibrary.PrintString` (`KismetStringLibrary.Conv_IntToString` _output_get))
      (bind (_direction _slowdown) (`Timeline|Target  slow fall`)
        (:`Update`
          (`SceneComponent.K2_SetRelativeRotation` :`self` (`self.Pivot`))
          (`KismetSystemLibrary.Delay` 0.5)
          (`self.K2_DestroyActor`))))))

(fn `UserConstructionScript`)