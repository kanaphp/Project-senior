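; BP_SpawnManager periodically spawns waves of random targets at BP_SpawnPoint locations in the level.
; A looping timer started on BeginPlay calls SpawnTarget by name every few seconds.
; Each wave gathers all spawn points, then spawns MaxSpawn random classes from AllTarget with a fixed rotation.
; Used points are removed from the local list to avoid repeats within a wave; earlier targets are not cleared.
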(event `self.ReceiveBeginPlay`
  (`KismetSystemLibrary.K2_SetTimer` null "Spawntarget" 4.5 true))

(fn `SpawnTarget`
  (locals (LocalSpawnReferences :type "Array of /Game/MyGame/Singburi/Blueprints/BP_SpawnPoint Object Reference") (LocalItem :type "/Game/MyGame/Singburi/Blueprints/BP_SpawnPoint Object Reference"))
  (`KismetSystemLibrary.PrintString` "Hello spawntarget activate")
  (bind _outactors (`GameplayStatics.GetAllActorsOfClass` "/Game/MyGame/Singburi/Blueprints/BP_SpawnPoint.BP_SpawnPoint_C"))
  (set `local.LocalSpawnReferences` _outactors)
  (for _ (range (`self.MaxSpawn`))
    (set `local.LocalItem` (`KismetArrayLibrary.Array_Random` (`local.LocalSpawnReferences`)))
    (`|SpawnActorFromClass` (`KismetArrayLibrary.Array_Random` (`self.AllTarget`)) (`KismetMathLibrary.MakeTransform` (`self.K2_GetActorLocation` (`local.LocalItem`)) (struct :`Yaw` 90.0)) "Undefined" "MultiplyWithRoot")
    (`KismetSystemLibrary.PrintString` "spawn!!")
    (`KismetArrayLibrary.Array_RemoveItem` (`local.LocalSpawnReferences`) (`local.LocalItem`))))

(fn `UserConstructionScript`)