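; Physical button board that shows a summary for five provinces (Pattani, Amnajchareon, Singburi, Srakeaw, Pichit) and has a Next button opening StartMap.
; Overlap boxes react only to BP_TestPress, sinking each button from its BeginPlay-cached position and restoring it on exit.
; A DoOnce per button, reset on exit, limits the press sound.
; It also gates the Pichit and Srakeaw summary calls, while the other actions fire on every overlap.
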(event `self.ReceiveBeginPlay`
  (`|ExecutionSequence`
    (:`then_0`
      (set `self.Pattani_Btn_Start` (`SceneComponent.RelativeLocation` (`self.Pattani_Btn`))))
    (:`then_1`
      (set `self.Amanj_Btn_Start` (`SceneComponent.RelativeLocation` (`self.Amnajchareon_Btn`))))
    (:`then_2`
      (set `self.Singburi_Btn_Start` (`SceneComponent.RelativeLocation` (`self.Singburi_Btn`))))
    (:`then_3`
      (set `self.Srakaew_Btn_Start` (`SceneComponent.RelativeLocation` (`self.Srakeaw_Btn`))))
    (:`then_4`
      (set `self.Pichit_Btn_Start` (`SceneComponent.RelativeLocation` (`self.Pichit_Btn`))))
    (:`then_5`
      (set `self.Next_Btn_Start` (`SceneComponent.RelativeLocation` (`self.Next_Btn`))))))

(event `self.Box4.OnComponentBeginOverlap`
  (params (OverlappedComponent :type "PrimitiveComponent Object Reference") (OtherActor :type "Actor Object Reference") (OtherComp :type "PrimitiveComponent Object Reference") (OtherBodyIndex :type Integer) (bFromSweep :type Boolean) (SweepResult :type "HitResult Structure (by ref)"))
  ; Show Singburi Summary
  (cast `/Game/MyGame/Question/BP_TestPress` OtherActor)
  (`|ExecutionSequence`
    (:`then_0`
      (`/Engine/EditorBlueprintResources/StandardMacros.DoOnce` false :!label _label
        (:`Completed`
          (`GameplayStatics.PlaySound2D` "/Game/MyGame/Sound/PressButton.PressButton" 1.0 1.0 0.0 null null))))
    (:`then_1`
      (`KismetSystemLibrary.MoveComponentTo` (`self.Singburi_Btn`) (- (`self.Singburi_Btn_Start`) (0.0 0.0 40.0)))
      (`self.ShowSingburi`))))

(event `self.Box1.OnComponentBeginOverlap`
  (params (OverlappedComponent :type "PrimitiveComponent Object Reference") (OtherActor :type "Actor Object Reference") (OtherComp :type "PrimitiveComponent Object Reference") (OtherBodyIndex :type Integer) (bFromSweep :type Boolean) (SweepResult :type "HitResult Structure (by ref)"))
  ; Show Pattani Summary
  (cast `/Game/MyGame/Question/BP_TestPress` OtherActor)
  (`|ExecutionSequence`
    (:`then_0`
      (`/Engine/EditorBlueprintResources/StandardMacros.DoOnce` false :!label _label_2
        (:`Completed`
          (`GameplayStatics.PlaySound2D` "/Game/MyGame/Sound/PressButton.PressButton" 1.0 1.0 0.0 null null))))
    (:`then_1`
      (`KismetSystemLibrary.MoveComponentTo` (`self.Pattani_Btn`) (- (`self.Pattani_Btn_Start`) (0.0 0.0 40.0)))
      (`self.ShowPattani`))))

(event `self.Box4.OnComponentEndOverlap`
  (params (OverlappedComponent :type "PrimitiveComponent Object Reference") (OtherActor :type "Actor Object Reference") (OtherComp :type "PrimitiveComponent Object Reference") (OtherBodyIndex :type Integer))
  ; Show Singburi Summary
  (cast `/Game/MyGame/Question/BP_TestPress` OtherActor)
  (`KismetSystemLibrary.MoveComponentTo` (`self.Singburi_Btn`) (`self.Singburi_Btn_Start`))
  (goto _label :!via `Reset`))

(event `self.Box1.OnComponentEndOverlap`
  (params (OverlappedComponent :type "PrimitiveComponent Object Reference") (OtherActor :type "Actor Object Reference") (OtherComp :type "PrimitiveComponent Object Reference") (OtherBodyIndex :type Integer))
  ; Show Pattani Summary
  (cast `/Game/MyGame/Question/BP_TestPress` OtherActor)
  (`KismetSystemLibrary.MoveComponentTo` (`self.Pattani_Btn`) (`self.Pattani_Btn_Start`))
  (goto _label_2 :!via `Reset`))

(event `self.Box3.OnComponentBeginOverlap`
  (params (OverlappedComponent :type "PrimitiveComponent Object Reference") (OtherActor :type "Actor Object Reference") (OtherComp :type "PrimitiveComponent Object Reference") (OtherBodyIndex :type Integer) (bFromSweep :type Boolean) (SweepResult :type "HitResult Structure (by ref)"))
  ; Show Amnajchareon Summary
  (cast `/Game/MyGame/Question/BP_TestPress` OtherActor)
  (`|ExecutionSequence`
    (:`then_0`
      (`/Engine/EditorBlueprintResources/StandardMacros.DoOnce` false :!label _label_3
        (:`Completed`
          (`GameplayStatics.PlaySound2D` "/Game/MyGame/Sound/PressButton.PressButton" 1.0 1.0 0.0 null null))))
    (:`then_1`
      (`KismetSystemLibrary.MoveComponentTo` (`self.Amnajchareon_Btn`) (- (`self.Amanj_Btn_Start`) (0.0 0.0 40.0)))
      (`self.ShowAmnajchareon`))))

(event `self.Box.OnComponentBeginOverlap`
  (params (OverlappedComponent :type "PrimitiveComponent Object Reference") (OtherActor :type "Actor Object Reference") (OtherComp :type "PrimitiveComponent Object Reference") (OtherBodyIndex :type Integer) (bFromSweep :type Boolean) (SweepResult :type "HitResult Structure (by ref)"))
  ; Show Pichit Summary
  (cast `/Game/MyGame/Question/BP_TestPress` OtherActor)
  (`|ExecutionSequence`
    (:`then_0`
      (`/Engine/EditorBlueprintResources/StandardMacros.DoOnce` false :!label _label_4
        (:`Completed`
          (`GameplayStatics.PlaySound2D` "/Game/MyGame/Sound/PressButton.PressButton" 1.0 1.0 0.0 null null)
          (`self.ShowPichit`))))
    (:`then_1`
      (`KismetSystemLibrary.MoveComponentTo` (`self.Pichit_Btn`) (- (`self.Pichit_Btn_Start`) (0.0 0.0 40.0))))))

(event `self.Box3.OnComponentEndOverlap`
  (params (OverlappedComponent :type "PrimitiveComponent Object Reference") (OtherActor :type "Actor Object Reference") (OtherComp :type "PrimitiveComponent Object Reference") (OtherBodyIndex :type Integer))
  ; Show Amnajchareon Summary
  (cast `/Game/MyGame/Question/BP_TestPress` OtherActor)
  (`KismetSystemLibrary.MoveComponentTo` (`self.Amnajchareon_Btn`) (`self.Amanj_Btn_Start`))
  (goto _label_3 :!via `Reset`))

(event `self.Box.OnComponentEndOverlap`
  (params (OverlappedComponent :type "PrimitiveComponent Object Reference") (OtherActor :type "Actor Object Reference") (OtherComp :type "PrimitiveComponent Object Reference") (OtherBodyIndex :type Integer))
  ; Show Pichit Summary
  (cast `/Game/MyGame/Question/BP_TestPress` OtherActor)
  (`KismetSystemLibrary.MoveComponentTo` (`self.Pichit_Btn`) (`self.Pichit_Btn_Start`))
  (goto _label_4 :!via `Reset`))

(event `self.Box2.OnComponentBeginOverlap`
  (params (OverlappedComponent :type "PrimitiveComponent Object Reference") (OtherActor :type "Actor Object Reference") (OtherComp :type "PrimitiveComponent Object Reference") (OtherBodyIndex :type Integer) (bFromSweep :type Boolean) (SweepResult :type "HitResult Structure (by ref)"))
  ; Next to Mainmenu
  (cast `/Game/MyGame/Question/BP_TestPress` OtherActor)
  (`|ExecutionSequence`
    (:`then_0`
      (`/Engine/EditorBlueprintResources/StandardMacros.DoOnce` false :!label _label_5
        (:`Completed`
          (`GameplayStatics.PlaySound2D` "/Game/MyGame/Sound/PressButton.PressButton" 1.0 1.0 0.0 null null))))
    (:`then_1`
      (`KismetSystemLibrary.MoveComponentTo` (`self.Next_Btn`) (- (`self.Next_Btn_Start`) (0.0 0.0 40.0)))
      (`GameplayStatics.OpenLevel` "StartMap"))))

(event `self.Box5.OnComponentBeginOverlap`
  (params (OverlappedComponent :type "PrimitiveComponent Object Reference") (OtherActor :type "Actor Object Reference") (OtherComp :type "PrimitiveComponent Object Reference") (OtherBodyIndex :type Integer) (bFromSweep :type Boolean) (SweepResult :type "HitResult Structure (by ref)"))
  ; Show Srakeaw Summary
  (cast `/Game/MyGame/Question/BP_TestPress` OtherActor)
  (`|ExecutionSequence`
    (:`then_0`
      (`/Engine/EditorBlueprintResources/StandardMacros.DoOnce` false :!label _label_6
        (:`Completed`
          (`GameplayStatics.PlaySound2D` "/Game/MyGame/Sound/PressButton.PressButton" 1.0 1.0 0.0 null null)
          (`self.ShowSrakeaw`))))
    (:`then_1`
      (`KismetSystemLibrary.MoveComponentTo` (`self.Srakeaw_Btn`) (- (`self.Srakaew_Btn_Start`) (0.0 0.0 40.0))))))

(event `self.Box2.OnComponentEndOverlap`
  (params (OverlappedComponent :type "PrimitiveComponent Object Reference") (OtherActor :type "Actor Object Reference") (OtherComp :type "PrimitiveComponent Object Reference") (OtherBodyIndex :type Integer))
  ; Next to Mainmenu
  (cast `/Game/MyGame/Question/BP_TestPress` OtherActor)
  (`KismetSystemLibrary.MoveComponentTo` (`self.Next_Btn`) (`self.Next_Btn_Start`))
  (goto _label_5 :!via `Reset`))

(event `self.Box5.OnComponentEndOverlap`
  (params (OverlappedComponent :type "PrimitiveComponent Object Reference") (OtherActor :type "Actor Object Reference") (OtherComp :type "PrimitiveComponent Object Reference") (OtherBodyIndex :type Integer))
  ; Show Srakeaw Summary
  (cast `/Game/MyGame/Question/BP_TestPress` OtherActor)
  (`KismetSystemLibrary.MoveComponentTo` (`self.Srakeaw_Btn`) (`self.Srakaew_Btn_Start`))
  (goto _label_6 :!via `Reset`))

(fn `UserConstructionScript`)